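; BP_TagSetter is an editor tool actor that edits the actor tags of an assigned Target actor.
; Its construction script either replaces the Target's tags with TargetTags, or adds or removes them depending on the Replace and Clear flags.
; It then resets Target, so each assignment acts as a one-shot operation.
; A debug event draws the connection to Target, and the actor destroys itself on BeginPlay.
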(event Custom|ShowConnections
  ;[0.1146 0.3359 1] Debug
  (Rendering|Debug|FlushPersistentDebugLines)
  (CallFunction|ShowConnection self (Variables|Default|GetTarget) "(R=1.000000,G=1.000000,B=1.000000,A=1.000000)" 3e+01))

(event EventBeginPlay
  (Actor|DestroyActor))

(fn ConstructionScript
  (Utilities|IsValid (Variables|Default|GetTarget)
    (:Is%20Valid
      (if (Variables|Default|GetReplace)
        (Variables|/Script/Engine.Actor|SetTags (Variables|Default|GetTarget) (Variables|Default|GetTargetTags))
        (else
          (for _array_element (Variables|Default|GetTargetTags)
            (if (Variables|Default|GetClear)
              (Utilities|Array|RemoveItem (Variables|/Script/Engine.Actor|GetTags (Variables|Default|GetTarget)) _array_element)
              (else
                (Utilities|Array|AddUnique (Variables|/Script/Engine.Actor|GetTags (Variables|Default|GetTarget)) _array_element))))))
      (Variables|Default|SetTarget 0))))