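; BP_KGPlayer is the player Blueprint for the kitty game, handling movement camera feedback, paw interaction and climbing.
; Each Tick, it starts a run or walk camera shake on the player camera manager while moving.
; Interacting plays a one-shot punch animation on the Paw.
; ClimbingComponent start and stop events switch CharacterMovement between Flying and Walking, so climbing uses the Flying mode.
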(event OnStartClimbing(ClimbingComponent)
  ;[0 0 0] Climb
  (Pawn|Components|CharacterMovement|SetMovementMode (Variables|Character|GetCharacterMovement) "MOVE_Flying" 0))

(event OnStopClimbing(ClimbingComponent)
  ;[0 0 0] Climb
  (Pawn|Components|CharacterMovement|SetMovementMode (Variables|Character|GetCharacterMovement) "MOVE_Walking" 0))

(event EventBeginPlay)

(event EventTick
  (params (DeltaSeconds :type Float%20%28single-precision%29))
  (bind _returnvalue (Game|GetPlayerCameraManager 0))
  (Utilities|IsValid _returnvalue
    (:Is%20Valid
      (if (Class|KGPlayer|IsMoving)
        (if (Class|KGPlayer|IsRunning)
          (CameraShakes|StartCameraShake _returnvalue "/Game/KittyGame/GameLogic/Blueprints/Camera/BP_RunCameraShake.BP_RunCameraShake_C" 1.0 "CameraLocal" "0, 0, 0")
          (else
            (CameraShakes|StartCameraShake _returnvalue "/Game/KittyGame/GameLogic/Blueprints/Camera/BP_WalkCameraShake.BP_WalkCameraShake_C" 1.0 "CameraLocal" "0, 0, 0")))))))

(event EventOnInteract
  ;[0 0 0] Interaction
  (Components|Animation|PlayAnimation (Variables|Default|GetPaw) "/Game/KittyGame/Assets/Animations/Cat/A_KittyPunch.A_KittyPunch" false))

(fn ConstructionScript)