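; BP_Radio is an interactable radio that the player cat can switch on and off to play positional music.
; On BeginPlay it caches the player and spawns an attenuated MetaSound at its location, kept alive and paused.
; A sphere overlap shows or hides a widget for the player.
; Interact plays the cat's paw punch, toggles pause or restarts stopped music, and switches the radio's mesh animation to match.
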(event OnComponentBeginOverlap(Sphere)
  (params (OverlappedComponent :type Primitive%20Component%20Object%20Reference) (OtherActor :type Actor%20Object%20Reference) (OtherComp :type Primitive%20Component%20Object%20Reference) (OtherBodyIndex :type Integer) (bFromSweep :type Boolean) (SweepResult :type Hit%20Result%20Structure%20%28by%20ref%29))
  (if (== OtherActor (Variables|Default|GetPlayerRef))
    (Rendering|SetVisibility (Variables|Default|GetWidget) true false)))

(event OnComponentEndOverlap(Sphere)
  (params (OverlappedComponent :type Primitive%20Component%20Object%20Reference) (OtherActor :type Actor%20Object%20Reference) (OtherComp :type Primitive%20Component%20Object%20Reference) (OtherBodyIndex :type Integer))
  (if (== OtherActor (Variables|Default|GetPlayerRef))
    (Rendering|SetVisibility (Variables|Default|GetWidget) false false)))

(event EventBeginPlay
  (bind _asbp_kgplayer (Utilities|Casting|CastToBP_KGPlayer (Game|GetPlayerCharacter 0)))
  (Variables|Default|SetPlayerRef _asbp_kgplayer)
  (bind _returnvalue (Audio|SpawnSoundatLocation "/Game/KittyGame/Assets/Audio/MetaSounds/MS_RadioMusic.MS_RadioMusic" (Transformation|GetActorLocation) "0, 0, 0" 1.0 1.0 0.0 "/Game/KittyGame/Assets/Audio/MetaSounds/SA_Radio.SA_Radio" 0 false))
  (bind _output_get (Variables|Default|SetMusic _returnvalue))
  (Class|AudioComponent|SetPaused _output_get true))

(fn ConstructionScript)

(fn Interact
  (params (Causer :type Actor%20Object%20Reference))
  (bind _music (Variables|Default|GetMusic))
  (Components|Animation|PlayAnimation (Variables|/Script/KittyGame.KGPlayer|GetPaw (Variables|Default|GetPlayerRef)) "/Game/KittyGame/Assets/Animations/Cat/AM_KittyPunh.AM_KittyPunh" false)
  (if (Audio|Components|Audio|IsPlaying _music)
    (if (Utilities|Enum|Equal(Enum) (Audio|Components|Audio|GetPlayState _music) "Paused")
      (Class|AudioComponent|SetPaused _music false)
      (Components|Animation|PlayAnimation (Variables|Default|GetSkeletalMesh) "/Game/KittyGame/Assets/Animations/Radio/SM_Radio__1__Anim.SM_Radio__1__Anim" false :!label _label)
      (else
        (Class|AudioComponent|SetPaused _music true)
        (Components|Animation|PlayAnimation (Variables|Default|GetSkeletalMesh) "/Game/KittyGame/Assets/Animations/Radio/SM_Radio_AnimMain.SM_Radio_AnimMain" false)))
    (else
      (Audio|Components|Audio|Play _music 0.0)
      (goto _label)))
  (return false))