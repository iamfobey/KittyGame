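; BP_DropItem is an interactable prop that the player's kitty can swat sideways.
; A sphere overlap shows and hides a widget as the player enters or leaves range.
; Interact plays a punch animation on the player's Paw and starts the Punch timeline.
; The timeline nudges the static mesh opposite the player capsule's right vector each update, scaled by its curve, without sweeping.
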(event OnComponentBeginOverlap(Sphere)
  (params (OverlappedComponent :type Primitive%20Component%20Object%20Reference) (OtherActor :type Actor%20Object%20Reference) (OtherComp :type Primitive%20Component%20Object%20Reference) (OtherBodyIndex :type Integer) (bFromSweep :type Boolean) (SweepResult :type Hit%20Result%20Structure%20%28by%20ref%29))
  (if (== OtherActor (Variables|Default|GetPlayerRef))
    (Rendering|SetVisibility (Variables|Default|GetWidget) true false)))

(event OnComponentEndOverlap(Sphere)
  (params (OverlappedComponent :type Primitive%20Component%20Object%20Reference) (OtherActor :type Actor%20Object%20Reference) (OtherComp :type Primitive%20Component%20Object%20Reference) (OtherBodyIndex :type Integer))
  (if (== OtherActor (Variables|Default|GetPlayerRef))
    (Rendering|SetVisibility (Variables|Default|GetWidget) false false)))

(event Custom|PunchItem
  (bind _newtrack_0 (Timeline|Punch PlayFromStart)
    (:Update
      (Transformation|AddWorldOffset (Variables|Default|GetStaticMesh) (* (* (Math|Vector|GetRightVector (Variables|/Script/Engine.Character|GetCapsuleComponent (Variables|Default|GetPlayerRef))) -1) (* _newtrack_0 2.0)) false false))))

(event EventBeginPlay
  (bind _asbp_kgplayer (Utilities|Casting|CastToBP_KGPlayer (Game|GetPlayerCharacter 0)))
  (Variables|Default|SetPlayerRef _asbp_kgplayer))

(fn ConstructionScript)

(fn Interact
  (params (Causer :type Actor%20Object%20Reference))
  (Components|Animation|PlayAnimation (Variables|/Script/KittyGame.KGPlayer|GetPaw (Variables|Default|GetPlayerRef)) "/Game/KittyGame/Assets/Animations/Cat/AM_KittyPunh.AM_KittyPunh" false)
  (CallFunction|PunchItem)
  (return false))